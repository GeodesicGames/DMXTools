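; DMX strobe light fixture Blueprint that drives a lens and point light from received DMX data, at runtime and in the editor.
; Custom begin play assigns components, materials, strobe effect table and DMX mapping to the parent fixture, then binds to the DMX subsystem.
; Received data is normalized and its strobe value pushed.
; Editor events reuse the same begin play, tick and receive logic, resetting lens materials first on begin play.
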(event Custom|CustomBeginPlay
  ;[1 1 1] Initialize Instance
  (Variables|Default|SetFixtureParameterUsage (Utilities|Struct|MakeStruct_ParameterUsage true false))
  (CallFunction|AssignFixtureComponents)
  (CallFunction|AssignFixtureMaterials)
  (CallFunction|AssignFixtureParameters)
  (CallFunction|AssignFixtureMapping)
  ;[1 1 1] Assign DMX event
  (EventDispatchers|BindEventtoOnProtocolReceived (|DMXSubsystem) (delegate Custom|CustomEvent_0))
  (|CallParentFunction))

(event Custom|CustomEvent_0
  (params (Protocol :type DMX%20Protocol%20Name%20Structure) (Universe :type Integer) (DMXBuffer :type Array%20of%20Bytes))
  ;[1 1 1] Push new data when received
  (CallFunction|GetDMXCurrentNormalizedData)
  (CallFunction|PushStrobe (Utilities|Struct|BreakStruct_DMXData (Variables|Default|GetDMXCurrentNormalizedData))))

(event Custom|CustomTick
  (params (Delta :type Float%20%28single-precision%29))
  ;[1 1 1] Editor
  (|CallParentFunction Delta))

(event Custom|CustomDMXReceiveEvent
  (params (Protocol :type DMX%20Protocol%20Name%20Structure) (Universe :type Integer) (DMXBuffer :type Array%20of%20Bytes))
  ;[1 1 1] Editor
  (CallFunction|CustomEvent0 Protocol Universe DMXBuffer))

(event EventEditorDMXReceive
  (params (Protocol :type DMX%20Protocol%20Name%20Structure) (Universe :type Integer) (DMXBuffer :type Array%20of%20Bytes))
  ;[1 1 1] Interface Calls
  (CallFunction|CustomDMXReceiveEvent Protocol Universe DMXBuffer))

(event EventEditorTick
  (params (Delta :type Float%20%28single-precision%29))
  ;[1 1 1] Interface Calls
  (CallFunction|CustomTick Delta))

(event EventEditorBeginPlay
  ;[1 1 1] Interface Calls
  ;;[1 1 1] Reset Materials if Change in Editor
  (CallFunction|InitializeMaterials)
  (CallFunction|CustomBeginPlay))

(event EventTick
  (params (DeltaSeconds :type Float%20%28single-precision%29))
  ;[1 1 1] Runtime
  (CallFunction|CustomTick DeltaSeconds))

(event EventBeginPlay
  ;[1 1 1] Runtime
  (CallFunction|CustomBeginPlay))

(fn ConstructionScript)

(fn AssignFixtureComponents
  (Variables|Default|SetFixtureLensComponent (Variables|Default|GetLens))
  (Variables|Default|SetFixturePointLightComponent (Variables|Default|GetPointLight)))

(fn AssignFixtureParameters
  (Variables|Default|SetFixtureIntensityMax (Variables|FixtureParameters|GetIntensityMax%20%28Lumens%29))
  (CallFunction|SetParameterEffectTable (Variables|Default|GetStrobeData) (Variables|EffectTables|GetStrobeEffectTable)))

(fn AssignFixtureMapping
  (Utilities|Struct|SetmembersinStruct_ParameterData (Variables|Default|GetStrobeData) (Variables|DMXNameMapping|GetStrobeFunctionName)))

(fn AssignFixtureMaterials
  (Variables|Default|SetFixtureLensMaterial "/DMXFixtures/Masters/M_Lens_Strobe_Master.M_Lens_Strobe_Master")
  (Variables|Default|SetFixtureLightMaterial "/DMXFixtures/Masters/M_Light_Strobe_Master.M_Light_Strobe_Master"))

(fn InitializeMaterials
  (Rendering|Material|SetMaterial (Variables|Default|GetLens) 0 "/DMXFixtures/Masters/M_Lens_Static_Master.M_Lens_Static_Master")
  (Utilities|Array|Clear (Variables|Default|GetDynamicMaterialArray)))