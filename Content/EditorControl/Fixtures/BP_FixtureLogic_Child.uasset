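; DMX stage-light fixture logic child Blueprint that overrides BeginPlay to remove the parent's DMX Game Instance dependency.
; BeginPlay reads the fixture patch, creates dynamic beam, lens and light-function materials, then sets initial state.
; Gobo and color wheel masks are baked into render-target disks, cached by effect table and fed to those materials.
; Optional dynamic occlusion uses looping, randomly timed line traces to drive beam height.
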(event Custom|CustomEvent
  (bind _beamdynamicmaterial (Variables|Default|GetBeamDynamicMaterial))
  (bind _fixturedynamicocclusioncomponent (Variables|Default|GetFixtureDynamicOcclusionComponent))
  (bind _fixturebeamcomponent (Variables|Default|GetFixtureBeamComponent))
  (bind _returnvalue (Transformation|GetWorldLocation _fixturedynamicocclusioncomponent))
  (bind _sphereradius (Collision|GetComponentBounds _fixturebeamcomponent))
  (bind _returnvalue_2 (* _sphereradius 2.0))
  ;[1 1 1] Set Dynamic occlusion
  (bind (_outhit _returnvalue_3) (Collision|LineTraceByChannel _returnvalue (+ _returnvalue (* (Math|Vector|GetUpVector _fixturedynamicocclusioncomponent) _returnvalue_2)) "TraceTypeQuery1" false 0 "None" false))
  (if _returnvalue_3
    (Rendering|Material|SetScalarParameterValue _beamdynamicmaterial "DMX Dynamic Height" (Math|Float|Clamp(Float) (- 1.0 (/ (.Distance (Collision|BreakHitResult _outhit)) _returnvalue_2))) :!class /Script/Engine.MaterialInstanceDynamic)
    (else
      (Rendering|Material|SetScalarParameterValue _beamdynamicmaterial "DMX Dynamic Height" 0.0 :!class /Script/Engine.MaterialInstanceDynamic))))

(event EventBeginPlay
  (bind _fixturebeammaterial (Variables|Default|GetFixtureBeamMaterial))
  (bind _fixturelensmaterial (Variables|Default|GetFixtureLensMaterial))
  (bind _fixturelightmaterial (Variables|Default|GetFixtureLightMaterial))
  (bind _fixturespotcomponent (Variables|Default|GetFixtureSpotComponent))
  (bind _fixturepointlightcomponent (Variables|Default|GetFixturePointLightComponent))
  ;[0 0.1395 1] Required to override DMX Game Instance dependency (See Default Fixture Logic BP)
  (Utilities|FlowControl|Sequence
    (:then_0
      (CallFunction|InitializeFixturePatch))
    (:then_1
      (Utilities|FlowControl|Sequence
        (:then_0
          ;[1 1 1] Set cast shadow on light
          (Utilities|IsValid _fixturespotcomponent
            (:Is%20Valid
              (Rendering|Components|Light|SetCastShadows _fixturespotcomponent (Variables|Default|GetCast%20Shadow)))))
        (:then_1
          (Utilities|IsValid _fixturepointlightcomponent
            (:Is%20Valid
              (Rendering|Components|Light|SetCastShadows _fixturepointlightcomponent (Variables|Default|GetCast%20Shadow)))))
        (:then_2
          ;[1 1 1] Create dynamic beam material
          (Utilities|IsValid _fixturebeammaterial
            (:Is%20Valid
              (bind _returnvalue (Rendering|Material|CreateDynamicMaterialInstance _fixturebeammaterial "None" :!class /Script/Engine.KismetMaterialLibrary))
              (bind _output_get (Variables|Default|SetBeamDynamicMaterial _returnvalue))
              (CallFunction|AssignDynamicMaterialstoComponents _output_get _fixturebeammaterial)
              (Utilities|Array|Add (Variables|Default|GetDynamicMaterialArray) (Variables|Default|GetBeamDynamicMaterial)))))
        (:then_3
          ;[1 1 1] Create dynamic Lens material
          (Utilities|IsValid _fixturelensmaterial
            (:Is%20Valid
              (bind _returnvalue_2 (Rendering|Material|CreateDynamicMaterialInstance _fixturelensmaterial "None" :!class /Script/Engine.KismetMaterialLibrary))
              (bind _output_get_2 (Variables|Default|SetLensDynamicMaterial _returnvalue_2))
              (CallFunction|AssignDynamicMaterialstoComponents _output_get_2 _fixturelensmaterial)
              (Utilities|Array|Add (Variables|Default|GetDynamicMaterialArray) (Variables|Default|GetLensDynamicMaterial)))))
        (:then_4
          ;[1 1 1] Create dynamic Light function material
          (if (Utilities|IsValid _fixturelightmaterial)
            (bind _returnvalue_3 (Rendering|Material|CreateDynamicMaterialInstance _fixturelightmaterial "None" :!class /Script/Engine.KismetMaterialLibrary))
            (bind _output_get_3 (Variables|Default|SetLightDynamicMaterial _returnvalue_3))
            (Utilities|Array|Add (Variables|Default|GetDynamicMaterialArray) _output_get_3)))
        (:then_5
          ;[1 1 1] Set Point light
          (if (and (Utilities|IsValid (Variables|Default|GetFixturePointLightComponent)) (Utilities|IsValid (Variables|Default|GetLightDynamicMaterial)))
            (Rendering|Components|Light|SetLightFunctionMaterial (Variables|Default|GetFixturePointLightComponent) (Variables|Default|GetLightDynamicMaterial))))
        (:then_6
          ;[1 1 1] Set Spot light
          (if (and (Utilities|IsValid (Variables|Default|GetFixtureSpotComponent)) (Utilities|IsValid (Variables|Default|GetLightDynamicMaterial)))
            (Rendering|Components|Light|SetLightFunctionMaterial (Variables|Default|GetFixtureSpotComponent) (Variables|Default|GetLightDynamicMaterial))
            (else
              (Development|PrintString "INVALID"))))
        (:then_7
          ;[1 1 1] Create and assign Gobo Disk
          (Utilities|IsValid (.DMXEffectTable (Utilities|Struct|BreakStruct_ParameterData (Variables|Default|GetGoboWheelData)))
            (:Is%20Valid
              (bind (_clean _frosted) (CallFunction|GetGoboDisk))
              (for _array_element (Variables|Default|GetDynamicMaterialArray)
                (Utilities|IsValid _array_element
                  (:Is%20Valid
                    (Rendering|Material|SetTextureParameterValue _array_element "DMX Gobo Disk" _clean)
                    (Rendering|Material|SetTextureParameterValue _array_element "DMX Gobo Disk Frosted" _frosted)
                    (Rendering|Material|SetScalarParameterValue _array_element "DMX Gobo Num Mask" (Math|Conversions|ToFloat(Integer) (Utilities|Array|Length (Variables|Default|GetGoboMaskArray))) :!class /Script/Engine.MaterialInstanceDynamic)))))))
        (:then_8
          ;[1 1 1] Create and assign color disk
          (Utilities|IsValid (.DMXEffectTable (Utilities|Struct|BreakStruct_ParameterData (Variables|Default|GetColorWheelData)))
            (:Is%20Valid
              (bind _disk_clean (CallFunction|GetColorDisk))
              (for _array_element_2 (Variables|Default|GetDynamicMaterialArray)
                (Utilities|IsValid _array_element_2
                  (:Is%20Valid
                    (Rendering|Material|SetTextureParameterValue _array_element_2 "DMX Color Disk" _disk_clean)
                    (Rendering|Material|SetScalarParameterValue _array_element_2 "DMX Color Num Mask" (Math|Conversions|ToFloat(Integer) (Utilities|Array|Length (Variables|Default|GetColorMaskArray))) :!class /Script/Engine.MaterialInstanceDynamic)))))))
        (:then_9
          ;[1 1 1] Set Dynamic occlusion
          (if (Math|Boolean|ANDBoolean (Variables|Default|GetUse%20Dynamic%20Occlusion) (Utilities|IsValid (Variables|Default|GetFixtureDynamicOcclusionComponent)) (Utilities|IsValid (Variables|Default|GetBeamDynamicMaterial)))
            (Utilities|Time|SetTimerbyEvent (delegate Custom|CustomEvent) (Math|Random|RandomFloatinRange 0.1 0.3) true)))
        (:then_10
          (CallFunction|SetInitialFixtureState))))))

(event EventTick
  (params (DeltaSeconds :type Float%20%28single-precision%29))
  (|CallParentFunction DeltaSeconds))

(fn ConstructionScript
  (|CallParentFunction))

(fn InitializeFixturePatch
  (bind _dmx (Variables|Default|GetDMX))
  (bind _returnvalue (Class|DMXComponent|GetFixturePatch _dmx))
  (Variables|Default|SetFixturePatch (Class|DMXEntityReferenceConversions|ToRef(FixturePatchObj) _returnvalue))
  (Variables|Default|SetFixturePatchFunctions (Class|DMXEntityFixturePatch|GetAllFunctionsinActiveMode _returnvalue)))

(fn GetColorDisk
  (CallFunction|PopulateColorArray)
  (for _array_element (Variables|Default|GetColorDiskArray)
    (if (== (.DMXEffectTable (Utilities|Struct|BreakStruct_ParameterData (Variables|Default|GetColorWheelData))) (.EffectTable (Utilities|Struct|BreakStruct_DiskData _array_element)))
      (Variables|Default|SetColorWheelArray (.DiskLinearColor (Utilities|Struct|BreakStruct_DiskData _array_element)))
      (return (.DiskClean (Utilities|Struct|BreakStruct_DiskData _array_element)))))
  (CallFunction|CreateColorDisk)
  (return 0))

(fn CreateColorDisk
  (bind _colormaskarray (Variables|Default|GetColorMaskArray))
  (bind _returnvalue (Utilities|Array|Length _colormaskarray))
  (bind _returnvalue_2 (Rendering|CreateRenderTarget2D 4096 256 "RTF_RGBA8" "(R=0.000000,G=0.000000,B=0.000000,A=1.000000)" true))
  (LocalVariables|SetDiskCleanRT _returnvalue_2)
  (bind _returnvalue_3 (Rendering|Material|CreateDynamicMaterialInstance "/DMXFixtures/Materials/M_BakeColorDisk.M_BakeColorDisk" "None" :!class /Script/Engine.KismetMaterialLibrary))
  (LocalVariables|SetBakeDiskMaterial _returnvalue_3)
  (Rendering|Material|SetTextureParameterValue (LocalVariables|GetBakeDiskMaterial) "RTImage" (LocalVariables|GetDiskCleanRT))
  (Rendering|Material|SetScalarParameterValue (LocalVariables|GetBakeDiskMaterial) "NumImages" (Math|Conversions|ToFloat(Integer) (Utilities|Array|Length (Variables|Default|GetColorMaskArray))) :!class /Script/Engine.MaterialInstanceDynamic)
  (for (_array_element _array_index) (Variables|Default|GetColorMaskArray)
    ;[1 1 1] Bake Color Disk
    (Rendering|Material|SetTextureParameterValue (LocalVariables|GetBakeDiskMaterial) "SourceImage" _array_element)
    (Rendering|Material|SetScalarParameterValue (LocalVariables|GetBakeDiskMaterial) "CurrentIndex" (Math|Conversions|ToFloat(Integer) _array_index) :!class /Script/Engine.MaterialInstanceDynamic)
    (Rendering|DrawMaterialtoRenderTarget (LocalVariables|GetDiskCleanRT) (LocalVariables|GetBakeDiskMaterial)))
  ;[1 1 1] Get color from texture
  (for (_ _array_index_2) (Variables|Default|GetColorMaskArray)
    (bind _returnvalue_4 (Rendering|ReadRenderTargetRawUV (LocalVariables|GetDiskCleanRT) (+ (/ (Math|Conversions|ToFloat(Integer) _array_index_2) (Math|Conversions|ToFloat(Integer) _returnvalue)) (/ 0.5 (Math|Conversions|ToFloat(Integer) _returnvalue))) 0.5))
    (Utilities|Array|Add (Variables|Default|GetColorWheelArray) (Utilities|Struct|MakeLinearColor (/ (.R (Utilities|Struct|BreakLinearColor _returnvalue_4)) 255.0) (/ (.G (Utilities|Struct|BreakLinearColor _returnvalue_4)) 255.0) (/ (.B (Utilities|Struct|BreakLinearColor _returnvalue_4)) 255.0) 1.0)))
  ;[1 1 1] Save
  (Utilities|Array|Add (Variables|Default|GetColorDiskArray) (Utilities|Struct|MakeStruct_DiskData (.DMXEffectTable (Utilities|Struct|BreakStruct_ParameterData (Variables|Default|GetColorWheelData))) (LocalVariables|GetDiskCleanRT) 0 (Variables|Default|GetColorWheelArray)))
  (return (LocalVariables|GetDiskCleanRT)))

(fn GetGoboDisk
  (CallFunction|PopulateGoboArray)
  (for _array_element (Variables|Default|GetGoboDiskArray)
    (if (== (.EffectTable (Utilities|Struct|BreakStruct_DiskData _array_element)) (.DMXEffectTable (Utilities|Struct|BreakStruct_ParameterData (Variables|Default|GetGoboWheelData))))
      (return (.DiskClean (Utilities|Struct|BreakStruct_DiskData _array_element)) (.DiskFrosted (Utilities|Struct|BreakStruct_DiskData _array_element)))))
  (bind (_diskclean _diskfrosted) (CallFunction|CreateGoboDisk))
  (return _diskclean _diskfrosted))

(fn CreateGoboDisk
  (bind _gobomaskarray (Variables|Default|GetGoboMaskArray))
  (bind _returnvalue (Rendering|CreateRenderTarget2D 4096 256 "RTF_R8"))
  (LocalVariables|SetDiskCleanRT _returnvalue)
  (bind _returnvalue_2 (Rendering|CreateRenderTarget2D 4096 256 "RTF_R8"))
  (LocalVariables|SetDiskFrostedRT _returnvalue_2)
  (bind _returnvalue_3 (Rendering|Material|CreateDynamicMaterialInstance "/DMXFixtures/Materials/M_BakeGoboDisk.M_BakeGoboDisk" "None" :!class /Script/Engine.KismetMaterialLibrary))
  (LocalVariables|SetBakeDiskMaterial _returnvalue_3)
  (Rendering|Material|SetTextureParameterValue (LocalVariables|GetBakeDiskMaterial) "RTImage" (LocalVariables|GetDiskCleanRT))
  (Rendering|Material|SetScalarParameterValue (LocalVariables|GetBakeDiskMaterial) "NumImages" (Math|Conversions|ToFloat(Integer) (Utilities|Array|Length _gobomaskarray)) :!class /Script/Engine.MaterialInstanceDynamic)
  (for (_array_element _array_index) _gobomaskarray
    ;[1 1 1] Bake Disk Clean
    (Rendering|Material|SetTextureParameterValue (LocalVariables|GetBakeDiskMaterial) "SourceImage" _array_element)
    (Rendering|Material|SetScalarParameterValue (LocalVariables|GetBakeDiskMaterial) "CurrentIndex" (Math|Conversions|ToFloat(Integer) _array_index) :!class /Script/Engine.MaterialInstanceDynamic)
    (Rendering|DrawMaterialtoRenderTarget (LocalVariables|GetDiskCleanRT) (LocalVariables|GetBakeDiskMaterial)))
  (Rendering|Material|SetTextureParameterValue (LocalVariables|GetBakeDiskMaterial) "RTImage" (LocalVariables|GetDiskFrostedRT))
  (Rendering|Material|SetScalarParameterValue (LocalVariables|GetBakeDiskMaterial) "BlurAmount" 0.08 :!class /Script/Engine.MaterialInstanceDynamic)
  (for (_array_element_2 _array_index_2) _gobomaskarray
    ;[1 1 1] Bake disk frosted
    (Rendering|Material|SetTextureParameterValue (LocalVariables|GetBakeDiskMaterial) "SourceImage" _array_element_2)
    (Rendering|Material|SetScalarParameterValue (LocalVariables|GetBakeDiskMaterial) "CurrentIndex" (Math|Conversions|ToFloat(Integer) _array_index_2) :!class /Script/Engine.MaterialInstanceDynamic)
    (Rendering|DrawMaterialtoRenderTarget (LocalVariables|GetDiskFrostedRT) (LocalVariables|GetBakeDiskMaterial)))
  ;[1 1 1] Save
  (Utilities|Array|Add (Variables|Default|GetGoboDiskArray) (Utilities|Struct|MakeStruct_DiskData (.DMXEffectTable (Utilities|Struct|BreakStruct_ParameterData (Variables|Default|GetGoboWheelData))) (LocalVariables|GetDiskCleanRT) (LocalVariables|GetDiskFrostedRT) (Utilities|Array|MakeArray)))
  (return (LocalVariables|GetDiskCleanRT) (LocalVariables|GetDiskFrostedRT)))