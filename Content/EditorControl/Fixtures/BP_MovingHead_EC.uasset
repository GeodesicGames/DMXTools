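; DMX moving head light fixture that drives pan, tilt, dimmer, strobe, gobo wheel, color wheel, frost and zoom from received DMX data.
; BeginPlay assigns components, materials, parameter ranges, effect tables and DMX function names, then binds to the DMX subsystem's protocol-received event.
; Each DMX update fetches normalized values and pushes them per parameter.
; Editor interface events reuse the runtime logic, resetting materials first, so the fixture also works in-editor.
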(event Custom|CustomBeginPlay
  ;[1 1 1] Initialize Instance
  (Variables|Default|SetFixtureParameterUsage (Utilities|Struct|MakeStruct_ParameterUsage true true true false true true true true true))
  (CallFunction|AssignFixtureComponents)
  (CallFunction|AssignFixtureMaterials)
  (CallFunction|AssignFixtureParameters)
  (CallFunction|AssignFixtureMapping)
  ;[1 1 1] Assign DMX event
  (EventDispatchers|BindEventtoOnProtocolReceived (|DMXSubsystem) (delegate Custom|CustomEvent_0))
  (|CallParentFunction))

(event Custom|CustomEvent_0
  (params (Protocol :type DMX%20Protocol%20Name%20Structure) (Universe :type Integer) (DMXBuffer :type Array%20of%20Bytes))
  (bind _dmxcurrentnormalizeddata (Variables|Default|GetDMXCurrentNormalizedData))
  (bind (_colorwheel _gobowheel _pan _tilt _dimmer _strobe _frost _zoom) (Utilities|Struct|BreakStruct_DMXData _dmxcurrentnormalizeddata))
  ;[1 1 1] Push new data when received
  (CallFunction|GetDMXCurrentNormalizedData)
  (Utilities|FlowControl|Sequence
    (:then_0
      (CallFunction|PushPan _pan))
    (:then_1
      (CallFunction|PushTilt _tilt))
    (:then_2
      (CallFunction|PushDimmer _dimmer))
    (:then_3
      (CallFunction|PushStrobe _strobe))
    (:then_4
      (CallFunction|PushGoboWheel _gobowheel))
    (:then_5
      (CallFunction|PushColorWheel _colorwheel))
    (:then_6
      (CallFunction|PushFrost _frost))
    (:then_7
      (CallFunction|PushZoom _zoom))))

(event Custom|CustomTick
  (params (Delta :type Float%20%28single-precision%29))
  ;[1 1 1] Editor
  (|CallParentFunction Delta))

(event Custom|CustomDMXReceiveEvent
  (params (Protocol :type DMX%20Protocol%20Name%20Structure) (Universe :type Integer) (DMXBuffer :type Array%20of%20Bytes))
  ;[1 1 1] Editor
  (CallFunction|CustomEvent0 Protocol Universe DMXBuffer))

(event EventEditorDMXReceive
  (params (Protocol :type DMX%20Protocol%20Name%20Structure) (Universe :type Integer) (DMXBuffer :type Array%20of%20Bytes))
  ;[1 1 1] Interface Calls
  (CallFunction|CustomDMXReceiveEvent Protocol Universe DMXBuffer))

(event EventEditorTick
  (params (Delta :type Float%20%28single-precision%29))
  ;[1 1 1] Interface Calls
  (CallFunction|CustomTick Delta))

(event EventEditorBeginPlay
  ;[1 1 1] Interface Calls
  ;;[1 1 1] Reset Materials if Change in Editor
  (CallFunction|InitializeMaterials)
  (CallFunction|CustomBeginPlay))

(event EventBeginPlay
  ;[1 1 1] Runtime
  (CallFunction|CustomBeginPlay))

(event EventTick
  (params (DeltaSeconds :type Float%20%28single-precision%29))
  ;[1 1 1] Runtime
  (CallFunction|CustomTick DeltaSeconds))

(fn ConstructionScript)

(fn AssignFixtureComponents
  (Variables|Default|SetFixtureSpotComponent (Variables|Default|GetSpotLight))
  (Variables|Default|SetFixtureYokeComponent (Variables|Default|GetYoke))
  (Variables|Default|SetFixtureHeadComponent (Variables|Default|GetHead))
  (Variables|Default|SetFixtureBeamComponent (Variables|Default|GetBeam))
  (Variables|Default|SetFixtureLensComponent (Variables|Default|GetLens))
  (Variables|Default|SetFixtureDynamicOcclusionComponent (Variables|Default|GetBeam)))

(fn AssignFixtureParameters
  (bind _tiltrange (Variables|FixtureParameters|GetTiltRange))
  (bind _panrange (Variables|FixtureParameters|GetPanRange))
  (bind _returnvalue (* _tiltrange 0.5))
  (bind _returnvalue_2 (* _panrange 0.5))
  (Variables|Default|SetFixtureColorTemp (Variables|FixtureParameters|GetColorTemperature%20%28K%29))
  (Variables|Default|SetFixtureIntensityMax (Variables|FixtureParameters|GetIntensityMax%20%28Lumens%29))
  (CallFunction|SetParameterRange (Variables|Default|GetPanData) _returnvalue_2 (* _returnvalue_2 -1.0))
  (CallFunction|SetParameterRange (Variables|Default|GetTiltData) (* _returnvalue -1.0) _returnvalue)
  (CallFunction|SetParameterRange (Variables|Default|GetZoomData) (Variables|FixtureParameters|GetZoom%20Min) (Variables|FixtureParameters|GetZoom%20Max))
  (CallFunction|SetParameterEffectTable (Variables|Default|GetStrobeData) (Variables|EffectTables|GetStrobeEffectTable))
  (CallFunction|SetParameterEffectTable (Variables|Default|GetGoboWheelData) (Variables|EffectTables|GetGoboEffectTable))
  (CallFunction|SetParameterEffectTable (Variables|Default|GetColorWheelData) (Variables|EffectTables|GetColorEffectTable)))

(fn AssignFixtureMapping
  (Utilities|Struct|SetmembersinStruct_ParameterData (Variables|Default|GetGoboWheelData) (Variables|DMXNameMapping|GetGoboWheelFunctionName))
  (Utilities|Struct|SetmembersinStruct_ParameterData (Variables|Default|GetColorWheelData) (Variables|DMXNameMapping|GetColorWheelFunctionName))
  (Utilities|Struct|SetmembersinStruct_ParameterData (Variables|Default|GetPanData) (Variables|DMXNameMapping|GetPanFunctionName))
  (Utilities|Struct|SetmembersinStruct_ParameterData (Variables|Default|GetTiltData) (Variables|DMXNameMapping|GetTiltFunctionName))
  (Utilities|Struct|SetmembersinStruct_ParameterData (Variables|Default|GetDimmerData) (Variables|DMXNameMapping|GetDimmerFunctionName))
  (Utilities|Struct|SetmembersinStruct_ParameterData (Variables|Default|GetZoomData) (Variables|DMXNameMapping|GetZoomFunctionName))
  (Utilities|Struct|SetmembersinStruct_ParameterData (Variables|Default|GetStrobeData) (Variables|DMXNameMapping|GetStrobeFunctionName))
  (Utilities|Struct|SetmembersinStruct_ParameterData (Variables|Default|GetFrostData) (Variables|DMXNameMapping|GetFrostFunctionName)))

(fn AssignFixtureMaterials
  (Variables|Default|SetFixtureBeamMaterial "/DMXFixtures/Masters/M_Beam_Master.M_Beam_Master")
  (Variables|Default|SetFixtureLensMaterial "/DMXFixtures/Masters/M_Lens_Master.M_Lens_Master")
  (Variables|Default|SetFixtureLightMaterial "/DMXFixtures/Masters/M_Light_Master.M_Light_Master"))

(fn InitializeMaterials
  (Rendering|Material|SetMaterial (Variables|Default|GetLens) 0 "/DMXFixtures/Masters/M_Lens_Master.M_Lens_Master")
  (Rendering|Material|SetMaterial (Variables|Default|GetBeam) 0 "/DMXFixtures/Masters/M_Beam_Master.M_Beam_Master")
  (Utilities|Array|Clear (Variables|Default|GetDynamicMaterialArray))
  (Utilities|Array|Clear (Variables|Default|GetColorDiskArray)))